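; Buff component that switches an attack amplification effect on and off for the actor that owns it.
; It overrides ApplyEffect and RemoveEffect, running the parent logic before sending AttAmpliticationMessage to the owner.
; Both calls pass Param01 of the current buff info as the amplification value, with a flag marking apply or remove, leaving the stat change to the owner.
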(fn ApplyEffect
  (|CallParentFunction)
  (Class|IBuffSystem|AttAmplitication(Message) (Components|GetOwner) (.Param01 (Utilities|Struct|BreakST_BuffInfo (Variables|Default|GetCurrentBuffInfo))) true))

(fn RemoveEffect
  (|CallParentFunction)
  (Class|IBuffSystem|AttAmplitication(Message) (Components|GetOwner) (.Param01 (Utilities|Struct|BreakST_BuffInfo (Variables|Default|GetCurrentBuffInfo))) false))