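; Buff component that raises its owner's attack while active, judging by its name and messages.
; It extends a parent buff's apply and remove effect functions, calling the parent first and then sending the owner an AttIncreaseMessage with an on/off flag.
; The amount comes from Param01 of the current buff info, and the owner is left to handle the actual stat change.
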(event EventApplyBuff
  (params (TableRowName :type Name :default "None")))

(fn ApplyEffect
  (|CallParentFunction)
  (Class|IBuffSystem|AttIncrease(Message) (Components|GetOwner) true (.Param01 (Utilities|Struct|BreakST_BuffInfo (Variables|Default|GetCurrentBuffInfo)))))

(fn RemoveEffect
  (|CallParentFunction)
  (Class|IBuffSystem|AttIncrease(Message) (Components|GetOwner) false (.Param01 (Utilities|Struct|BreakST_BuffInfo (Variables|Default|GetCurrentBuffInfo)))))