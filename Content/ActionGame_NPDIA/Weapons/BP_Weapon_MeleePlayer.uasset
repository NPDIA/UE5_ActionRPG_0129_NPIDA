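; Player melee weapon Blueprint that deals damage to actors its capsule collider begins overlapping.
; Overlaps apply damage only while the weapon is active and its owner controller is valid, skipping that controller's own pawn and crediting it as instigator.
; A DamageActors list limits each actor to one hit per melee check, and the BeginMeleeCheck override clears it after calling the parent.
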(event OnComponentBeginOverlap(Col_Capsule)
  (params (OverlappedComponent :type Primitive%20Component%20Object%20Reference) (OtherActor :type Actor%20Object%20Reference) (OtherComp :type Primitive%20Component%20Object%20Reference) (OtherBodyIndex :type Integer) (bFromSweep :type Boolean) (SweepResult :type Hit%20Result%20Structure%20%28by%20ref%29))
  (Variables|Default|GetRefOwnerController
    (:then
      (if (Math|Boolean|ANDBoolean (not (Utilities|Set|Contains (Variables|Default|GetDamageActors) OtherActor)) (Variables|Default|GetIsActiveWeapon) (!= (Pawn|GetControlledPawn (Variables|Default|GetRefOwnerController)) OtherActor))
        (Utilities|Set|Add (Variables|Default|GetDamageActors) OtherActor)
        (Game|Damage|ApplyDamage OtherActor (Variables|Default|GetDamage) (Variables|Default|GetRefOwnerController) 0)))
    (:else)))

(event EventBeginMeleeCheck
  (|CallParentFunction)
  (Utilities|Set|Clear (Variables|Default|GetDamageActors)))

(fn ConstructionScript
  (|CallParentFunction))