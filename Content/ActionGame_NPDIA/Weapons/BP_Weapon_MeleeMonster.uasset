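; BP_Weapon_MeleeMonster is a monster melee weapon that damages the player on contact.
; When its capsule collision begins overlapping an actor tagged Player while the weapon is active, it applies damage credited to the owner's controller.
; A timestamp check enforces a one-second cooldown between hits.
; The construction script only calls its parent.
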(event OnComponentBeginOverlap(Col_Capsule)
  (params (OverlappedComponent :type Primitive%20Component%20Object%20Reference) (OtherActor :type Actor%20Object%20Reference) (OtherComp :type Primitive%20Component%20Object%20Reference) (OtherBodyIndex :type Integer) (bFromSweep :type Boolean) (SweepResult :type Hit%20Result%20Structure%20%28by%20ref%29))
  (if (Math|Boolean|ANDBoolean (Actor|ActorHasTag OtherActor "Player") (> (Utilities|Time|GetGameTimeinSeconds) (+ (Variables|Default|GetLastOverlapTime) 1.0)) (Variables|Default|GetIsActiveWeapon))
    (Variables|Default|SetLastOverlapTime (Utilities|Time|GetGameTimeinSeconds))
    (Game|Damage|ApplyDamage OtherActor (Variables|Default|GetDamage) (Variables|Default|GetRefOwnerController) self)))

(fn ConstructionScript
  (|CallParentFunction))