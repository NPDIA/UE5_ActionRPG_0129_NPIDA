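; Base monster character that loads its stats from MonsterTable, starts a behavior tree through AC_Monster and fights with a spawned, socket-attached weapon.
; MeleeAttack plays the attack montage and returns its length, while melee weapon activation is toggled separately.
; Damage knocks it away from the instigator and reduces HP.
; Death plays a montage, spawns table-driven random item and experience pickups, then calls OnDie.
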(event Custom|PlayAttackMTG
  (Animation|Montage|PlayMontage (Variables|Character|GetMesh) (Variables|EssentialSetup|GetAttackMTG)))

(event Custom|InitInfo
  (params (TableID :type Name))
  (Variables|Default|SetIsAlive true)
  (bind _returnvalue (Utilities|GetDataTableRow "/Game/ActionGame_NPDIA/Tables/MonsterTable.MonsterTable" TableID)
    (:then
      (Variables|Default|SetMonsterData _returnvalue)
      (bind _output_get (Variables|Default|SetMaxHP (.MaxHP (Utilities|Struct|BreakST_MonsterData _returnvalue))))
      (Variables|Default|SetCurrentHP _output_get))))

(event Custom|HiddenMesh
  (Rendering|SetVisibility (Variables|Character|GetMesh) false false)
  (Actor|DestroyActor (Variables|Default|GetCurrentWeapon)))

(event EventBeginPlay
  (if (Utilities|IsValidClass (Variables|Default|GetEquipWeaponClass))
    (bind _returnvalue (Game|SpawnActorfromClass (Variables|Default|GetEquipWeaponClass) (Transformation|GetActorTransform) "AlwaysSpawn" "MultiplyWithRoot" 0 self))
    (bind _output_get (Variables|Default|SetCurrentWeapon _returnvalue))
    (Transformation|AttachComponentToComponent _output_get (Variables|Character|GetMesh) (Variables|Default|GetWaeponSocket) "SnapToTarget" "SnapToTarget" "SnapToTarget" true)
    (Animation|Montage|PlayMontage (Variables|Character|GetMesh) (Variables|EssentialSetup|GetSpawnMTG))))

(event EventStartAI
  (CallFunction|InitInfo "None")
  (bind _asac_monster (Utilities|Casting|CastToAC_Monster (Pawn|GetController)))
  (Default|StartAIController _asac_monster (Variables|EssentialSetup|GetBlackboradAsset) (Variables|EssentialSetup|GetBtAssets)))

(event EventSetCurrentWeaponActive
  (params (IsActive :type Boolean))
  (bind _asbp_weapon_melee_attack_base (Utilities|Casting|CastToBP_Weapon_MeleeAttackBase (Variables|Default|GetCurrentWeapon)))
  (Variables|/Game/ActionGame_NPDIA/Weapons/BP_Weapon_MeleeAttackBase.BP_Weapon_MeleeAttackBase_C|SetIsActiveWeapon _asbp_weapon_melee_attack_base IsActive))

(event Custom|OnDieProcess
  (Variables|Default|SetIsAlive false)
  (Animation|StopAnimMontage (Animation|GetCurrentMontage :!class /Script/Engine.Character))
  (Animation|Montage|PlayMontage (Variables|Character|GetMesh) (Variables|EssentialSetup|GetDieMontage)
    (:then
      (Utilities|FlowControl|Delay 0.5) ; Event에서만 사용 가능
      (CallFunction|DropItem)
      (Default|CallOnDie self))))

(event Custom|DropItem
  (bind _monsterdata (Variables|Default|GetMonsterData))
  (bind (_monsterclass _monstername _maxhp _attack _defense _dropitemdata _dropexp) (Utilities|Struct|BreakST_MonsterData _monsterdata))
  (Utilities|FlowControl|Sequence
    (:then_0
      (for _array_element _dropitemdata
        (if (< (Math|Random|RandomFloatinRange 0.0 1.0) (.Rate (Utilities|Struct|BreakST_DropTable _array_element)))
          (bind _returnvalue (Game|SpawnActorfromClass "/Game/ActionGame_NPDIA/Item/BP_DropItemBase.BP_DropItemBase_C" (Transformation|GetActorTransform) "Undefined" "MultiplyWithRoot" 0 0))
          (Default|SetDropItemData _returnvalue (Utilities|Struct|MakeST_DropItemData (.ItemID (Utilities|Struct|BreakST_DropTable _array_element)) "NewEnumerator1" (Math|Random|RandomIntegerinRange (.MinAmount (Utilities|Struct|BreakST_DropTable _array_element)) (.MaxAmount (Utilities|Struct|BreakST_DropTable _array_element))) (.Countable (Utilities|Struct|BreakST_DropTable _array_element)))))))
    (:then_1
      (for _array_element_2 _dropexp
        (bind _returnvalue_2 (Game|SpawnActorfromClass "/Game/ActionGame_NPDIA/Item/BP_DropItemBase.BP_DropItemBase_C" (Transformation|GetActorTransform) "Undefined" "MultiplyWithRoot" 0 0))
        (Default|SetDropItemData _returnvalue_2 (Utilities|Struct|MakeST_DropItemData 0 "NewEnumerator0" _array_element_2 false))))))

(event Game|Damage|EventAnyDamage
  (params (Damage :type Float%20%28single-precision%29) (DamageType :type Damage%20Type%20Object%20Reference) (InstigatedBy :type Controller%20Object%20Reference) (DamageCauser :type Actor%20Object%20Reference))
  (if (Variables|Default|GetIsAlive)
    (Character|LaunchCharacter (* (Math|Vector|Normalize (- (Transformation|GetActorLocation) (Transformation|GetActorLocation (Pawn|GetControlledPawn InstigatedBy)))) 1.5e+03) false false)
    (bind _output_get (Variables|Default|SetCurrentHP (Math|Float|Clamp(Float) (- (Variables|Default|GetCurrentHP) Damage) 0.0 (Variables|Default|GetMaxHP))))
    (if (<= _output_get 1.0)
      (CallFunction|OnDieProcess))))

(fn ConstructionScript)

(fn MeleeAttack
  (CallFunction|PlayAttackMTG)
  (return (Animation|GetPlayLength (Variables|EssentialSetup|GetAttackMTG))))

(fn CreateRandomItemData)

(fn GetCurrentWeapon
  (Utilities|Casting|CastToBP_WeaponBase (Variables|Default|GetCurrentWeapon))
  (return 0))

(fn GetIsAlive
  (return (Variables|Default|GetIsAlive)))