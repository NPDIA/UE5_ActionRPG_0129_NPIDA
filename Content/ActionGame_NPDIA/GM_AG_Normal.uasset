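; Game mode for the normal mode of the action game, running the match countdown timer.
; StartPlayTimer sets the game time to five minutes and starts a looping one-second timer.
; Each tick decrements the time and calls the countdown event dispatcher.
; When time runs out, it clamps to zero, clears the timer and only prints a GameOver message.
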(event Custom|StartPlayTimer
  (Variables|Default|SetGameTime 300)
  (bind _returnvalue (Utilities|Time|SetTimerbyEvent (delegate Custom|CountDown) 1.0 true))
  (Variables|Default|SetTimerHandle _returnvalue))

(event Custom|CountDown
  (Math|Integer|DecrementInt (Variables|Default|GetGameTime)
    (:%20%20
      (Default|CallEDCountDown)
      (if (< (Variables|Default|GetGameTime) 1)
        (Variables|Default|SetGameTime 0)
        (Utilities|Time|ClearandInvalidateTimerbyHandle (Variables|Default|GetTimerHandle))
        (Development|PrintString "GameOver")))))

(fn ConstructionScript)