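; Base player character for an action game, handling movement, sword combo attacks, stats and item pickup.
; Init spawns and attaches the sword, creates the HUD, seeds HP/MP/EXP and initializes the inventory component.
; ChangeState clamps stats and broadcasts percentages; damage subtracts fixed HP, ignoring the incoming amount, while auto-pickups grant EXP.
; Attacks chain montage sections during combo windows; F stores overlapped items, and I toggles inventory alongside ground input mapping.
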(event OnComponentBeginOverlap(PickupBox)
  (params (OverlappedComponent :type Primitive%20Component%20Object%20Reference) (OtherActor :type Actor%20Object%20Reference) (OtherComp :type Primitive%20Component%20Object%20Reference) (OtherBodyIndex :type Integer) (bFromSweep :type Boolean) (SweepResult :type Hit%20Result%20Structure%20%28by%20ref%29))
  (Variables|Default|SetPickupTarget OtherActor))

(event OnComponentEndOverlap(PickupBox)
  (params (OverlappedComponent :type Primitive%20Component%20Object%20Reference) (OtherActor :type Actor%20Object%20Reference) (OtherComp :type Primitive%20Component%20Object%20Reference) (OtherBodyIndex :type Integer))
  (bind _pickupbox (Variables|Default|GetPickupBox))
  (bind _overlappingactors (Collision|GetOverlappingActors _pickupbox "/Game/ActionGame_NPDIA/Item/BP_DropItemBase.BP_DropItemBase_C" :!class /Script/Engine.PrimitiveComponent))
  (if (== OtherActor (Variables|Default|GetPickupTarget))
    (Variables|Default|SetPickupTarget 0)
    (if (> (Utilities|Array|Length _overlappingactors) 0)
      (Variables|Default|SetPickupTarget (Utilities|Array|Get(acopy) _overlappingactors)))))

(event Custom|MoveForward
  (Pawn|Input|AddMovementInput (Math|Vector|GetForwardVector (Math|Rotator|MakeRotator 0.0 0.0 (.yaw (Pawn|GetControlRotation :!class /Script/Engine.Pawn)))) 1.0 false))

(event Custom|ChangeState
  (params (ChangeHp :type Float%20%28double-precision%29) (ChangeMp :type Float%20%28double-precision%29) (ChangeExp :type Float%20%28double-precision%29))
  (Variables|State|SetCurrentHp (Math|Float|Clamp(Float) (+ (Variables|State|GetCurrentHp) ChangeHp) 0.0 (Variables|State|GetMaxHp)))
  (Variables|State|SetCurrentMp (Math|Float|Clamp(Float) (+ (Variables|State|GetCurrentMp) ChangeMp) 0.0 (Variables|State|GetMaxMp)))
  (Variables|State|SetCurrentExp (Math|Float|Clamp(Float) (+ (Variables|State|GetCurrentExp) ChangeExp) 0.0 (Variables|State|GetMaxExp)))
  (Default|CallEDChangeState (/ (Variables|State|GetCurrentHp) (Variables|State|GetMaxHp)) (/ (Variables|State|GetCurrentMp) (Variables|State|GetMaxMp)) (/ (Variables|State|GetCurrentExp) (Variables|State|GetMaxExp))))

(event Custom|InputMappingGround
  (params (NewActive :type Boolean))
  (bind _as플레이어_컨트롤러 (Utilities|Casting|CastToPlayerController (Pawn|GetController)))
  (Utilities|IsValid (PlayerController|LocalPlayerSubsystems|GetEnhancedInputLocalPlayerSubsystem _as플레이어_컨트롤러)
    (:Is%20Valid
      (if NewActive
        (Input|AddMappingContext (PlayerController|LocalPlayerSubsystems|GetEnhancedInputLocalPlayerSubsystem _as플레이어_컨트롤러) "/Game/ActionGame_NPDIA/Input/IMC_AG_GroundCharacter.IMC_AG_GroundCharacter" 0 "(bIgnoreAllPressedKeysUntilRelease=True,bForceImmediately=False,bNotifyUserSettings=False)")
        (else
          (Input|RemoveMappingContext (PlayerController|LocalPlayerSubsystems|GetEnhancedInputLocalPlayerSubsystem _as플레이어_컨트롤러) "/Game/ActionGame_NPDIA/Input/IMC_AG_GroundCharacter.IMC_AG_GroundCharacter" "(bIgnoreAllPressedKeysUntilRelease=True,bForceImmediately=False,bNotifyUserSettings=False)"))))))

(event Custom|Character_Init
  (bind _self self)
  (Utilities|FlowControl|Sequence
    (:then_0
      (bind _returnvalue (Game|SpawnActorfromClass "/Game/ActionGame_NPDIA/Player/BP_Player_Sword.BP_Player_Sword_C" (Transformation|GetActorTransform) "AlwaysSpawn" "MultiplyWithRoot" _self _self))
      (bind _output_get (Variables|Default|SetCurrentWeapon _returnvalue))
      (Default|EquipWeapon _output_get (Pawn|GetController) 1e+01)
      (Transformation|AttachComponentToComponent _output_get (Variables|Character|GetMesh) "sword_bottom" "SnapToTarget" "SnapToTarget" "SnapToTarget" true))
    (:then_1
      (CallFunction|InputMappingGround true)
      (bind _aspc_ag_base_controller (Utilities|Casting|CastToPC_AG_BaseController (Game|GetPlayerController 0)))
      (Default|CreateHUD _aspc_ag_base_controller))
    (:then_2
      (bind _output_get_2 (Variables|State|SetMaxHp 5e+02))
      (Variables|State|SetCurrentHp _output_get_2)
      (bind _output_get_3 (Variables|State|SetMaxMp 1e+02))
      (Variables|State|SetCurrentMp _output_get_3)
      (Variables|State|SetMaxExp 5e+02)
      (Variables|State|SetCurrentExp 0.0)
      (CallFunction|ChangeState 0.0 0.0 0.0))
    (:then_3
      (Default|InitInventory (Variables|Default|GetBPC_Inventory)))))

(event Input|EnhancedActionEvents|EnhancedInputActionIA_AG_Attack
  (params (ActionValue :type Boolean) (ElapsedSeconds :type Float%20%28double-precision%29) (TriggeredSeconds :type Float%20%28double-precision%29) (InputAction :type Input%20Action%20Object%20Reference :default "/Game/ActionGame_NPDIA/Input/IA_AG_Attack.IA_AG_Attack"))
  (bind _mesh (Variables|Character|GetMesh))
  (bind _returnvalue (Components|SkeletalMesh|GetAnimInstance _mesh))
  (bind _returnvalue_2 (Animation|Montage|GetCurrentActiveMontage _returnvalue))
  (:Started
    (if (Variables|Default|GetEnableAttack)
      (Variables|Default|SetEnableAttack false)
      (Variables|Default|SetEnableMove false)
      (Animation|Montage|PlayMontage (Variables|Character|GetMesh) "/Game/ActionGame_NPDIA/Player/MTG_AG_ComboAttack.MTG_AG_ComboAttack"
        (:OnCompleted
          (Variables|Default|SetEnableAttack true)
          (Variables|Default|SetEnableMove true)))
      (elif (Variables|Default|GetEnableCombo)
        (Class|AnimInstance|MontageSetNextSection _returnvalue (Animation|Montage|MontageGetCurrentSection _returnvalue _returnvalue_2) (Variables|Default|GetNextSectionName) _returnvalue_2)))))

(event Input|EnhancedActionEvents|EnhancedInputActionIA_AG_Locomotion
  (params (ActionValue :type Vector%202D%20Structure) (ElapsedSeconds :type Float%20%28double-precision%29) (TriggeredSeconds :type Float%20%28double-precision%29) (InputAction :type Input%20Action%20Object%20Reference :default "/Game/ActionGame_NPDIA/Input/IA_AG_Locomotion.IA_AG_Locomotion"))
  (bind _returnvalue (Pawn|GetControlRotation :!class /Script/Engine.Pawn))
  (if (Variables|Default|GetEnableMove)
    (Pawn|Input|AddMovementInput (Math|Vector|GetRightVector (Math|Rotator|MakeRotator (.roll _returnvalue) 0.0 (.yaw _returnvalue))) (.x ActionValue) false)
    (Pawn|Input|AddMovementInput (Math|Vector|GetForwardVector (Math|Rotator|MakeRotator 0.0 0.0 (.yaw _returnvalue))) (.y ActionValue) false)))

(event Input|EnhancedActionEvents|EnhancedInputActionIA_AG_CamRotate
  (params (ActionValue :type Vector%202D%20Structure) (ElapsedSeconds :type Float%20%28double-precision%29) (TriggeredSeconds :type Float%20%28double-precision%29) (InputAction :type Input%20Action%20Object%20Reference :default "/Game/ActionGame_NPDIA/Input/IA_AG_CamRotate.IA_AG_CamRotate"))
  (Pawn|Input|AddControllerYawInput (.x ActionValue))
  (Pawn|Input|AddControllerPitchInput (.y ActionValue)))

(event Game|Damage|EventAnyDamage
  (params (Damage :type Float%20%28single-precision%29) (DamageType :type Damage%20Type%20Object%20Reference) (InstigatedBy :type Controller%20Object%20Reference) (DamageCauser :type Actor%20Object%20Reference))
  (CallFunction|ChangeState -1e+02 0.0 0.0)
  (Development|PrintString (Utilities|String|Append "Damage : " (Utilities|String|ToString(Float) Damage) ", DamageType : " (Utilities|GetDisplayName DamageType) ", Instigated By : " (Utilities|GetDisplayName InstigatedBy) ", Damage Causer : " (Utilities|GetDisplayName DamageCauser)) true true "(R=0.000000,G=0.660000,B=1.000000,A=1.000000)" 5.0))

(event EventAutoPickup
  (params (DropItemData :type ST%20Drop%20Item%20Data%20Structure))
  (CallFunction|ChangeState 0.0 0.0 (Math|Conversions|ToFloat(Integer) (.amount DropItemData))))

(event Input|KeyboardEvents|F
  (params (Key :type Key%20Structure :default "None"))
  (:Pressed
    (bind _pickuptarget (Variables|Default|GetPickupTarget)
      (:then
        (bind _dropitemdata (Class|IPickupItem|PickupItem(Message) _pickuptarget))
        (bind _pickupresult (Default|TryAddItem (Variables|Default|GetBPC_Inventory) _dropitemdata))
        (switch Utilities|FlowControl|Switch|SwitchonE_PickupResult _pickupresult
          (:NewEnumerator0
            (Actor|DestroyActor _pickuptarget))
          (:NewEnumerator1
            (Development|PrintString "Inventory is Full!!"))
          (:NewEnumerator2
            (Development|PrintString "Unknowned Error!!"))))
      (:else))))

(event Input|KeyboardEvents|I
  (params (Key :type Key%20Structure :default "None"))
  (bind _bpc_inventory (Variables|Default|GetBPC_Inventory))
  (bind _bpc_inventory_2 (Variables|Default|GetBPC_Inventory))
  (:Pressed
    (Variables|/Game/ActionGame_NPDIA/Item/BPC_Inventory.BPC_Inventory_C|GetInventoryWidget _bpc_inventory
      (:then
        _)
      (:else
        (Default|CreateInventoryWdiget _bpc_inventory)))
    (if (Variables|/Game/ActionGame_NPDIA/Item/BPC_Inventory.BPC_Inventory_C|GetIsOpen _bpc_inventory)
      (Default|CloseInventoryWidget _bpc_inventory_2)
      (CallFunction|InputMappingGround true)
      (else
        (Default|OpenInventoryWidget _bpc_inventory_2)
        (CallFunction|InputMappingGround false)))))

(fn ConstructionScript)

(fn PickupItem
  (return ""))